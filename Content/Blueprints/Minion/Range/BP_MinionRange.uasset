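; BP_MinionRange is the ranged minion character, which hides its left and right weapon bones on spawn.
; It binds to its HealthComponent death event at BeginPlay.
; On death it detaches its controller, disables capsule collision, ragdolls the mesh through physics simulation and deactivates the health component.
; A random roll then gives a small chance to drop an ammo pickup at its location.
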(event Custom|OnActorDeath_Event_0
  (bind _mesh (Variables|Character|GetMesh))
  (Class|Pawn|DetachfromControllerPendingDestroy)
  (Collision|SetCollisionEnabled (Variables|Default|GetCapsuleComponent) "NoCollision")
  (Collision|SetCollisionEnabled _mesh "QueryAndPhysics")
  (Physics|SetSimulatePhysics _mesh true)
  (Components|Activation|SetActive (Variables|Default|GetHealthComponent) false false)
  ;[1 1 1] Chance To Spawn Ammo
  (if (< (Math|Random|RandomFloat) 0.1)
    (Game|SpawnActorfromClass "/Game/Blueprints/BP_AmmoPickup.BP_AmmoPickup_C" (Transformation|GetActorTransform) "Undefined" 0 0)))

(event EventBeginPlay
  (EventDispatchers|AssignOnActorDeath (Variables|Default|GetHealthComponent) (delegate Custom|OnActorDeath_Event_0))
  (Components|SkinnedMesh|HideBonebyName (Variables|Character|GetMesh) "weapon_l" "PBO_None")
  (Components|SkinnedMesh|HideBonebyName (Variables|Character|GetMesh) "weapon_r" "PBO_None"))

(fn ConstructionScript)