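; BP_LaserCage is a boss-fight laser cage that stays hidden until StartCage is called.
; StartCage reveals it, switches off its four BP_Lasers child actors and plays an ActorSequence animation.
; When the sequence finishes, a bound OnFinished event switches all four lasers on through a helper that casts each child actor to BP_Lasers.
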(event Custom|OnFinished_Event_0
  (CallFunction|ActivateLaser (Variables|Default|GetBP_Lasers) true)
  (CallFunction|ActivateLaser (Variables|Default|GetBP_Lasers1) true)
  (CallFunction|ActivateLaser (Variables|Default|GetBP_Lasers2) true)
  (CallFunction|ActivateLaser (Variables|Default|GetBP_Lasers3) true))

(event Custom|StartCage
  (Sequencer|Player|Play (Variables|/Script/ActorSequence.ActorSequenceComponent|GetSequencePlayer (Variables|Default|GetActorSequence)) :!class /Script/MovieScene.MovieSceneSequencePlayer)
  (Rendering|SetActorHiddenInGame false)
  (CallFunction|ActivateLaser (Variables|Default|GetBP_Lasers) false)
  (CallFunction|ActivateLaser (Variables|Default|GetBP_Lasers1) false)
  (CallFunction|ActivateLaser (Variables|Default|GetBP_Lasers2) false)
  (CallFunction|ActivateLaser (Variables|Default|GetBP_Lasers3) false))

(event EventBeginPlay
  (EventDispatchers|AssignOnFinished (Variables|/Script/ActorSequence.ActorSequenceComponent|GetSequencePlayer (Variables|Default|GetActorSequence)) (delegate Custom|OnFinished_Event_0))
  (Rendering|SetActorHiddenInGame true))

(fn ConstructionScript)

(fn ActivateLaser
  (params (Laser :type Child%20Actor%20Component%20Object%20Reference) (Active :type Boolean))
  (bind _asbp_lasers (Utilities|Casting|CastToBP_Lasers (Variables|/Script/Engine.ChildActorComponent|GetChildActor Laser)))
  (Default|ActivateLasers _asbp_lasers Active))