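; BP_Laser is a boss attack laser actor that projects a colored beam along its forward vector.
; On BeginPlay it applies LaserColor to the Laser and LaserImpact effects.
; Each tick a Camera-channel line trace, debug-drawn per frame, feeds the beam's LaserEnd parameter with the hit point, or maximum Distance on a miss.
; The impact effect moves to the hit point and shows only on a blocking hit; no damage is applied here.
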(event EventBeginPlay
  (Effects|Components|ParticleSystem|SetColorParameter (Variables|Default|GetLaser) "Color" (Variables|Default|GetLaserColor)))

(event EventTick
  (params (DeltaSeconds :type Float%20%28single-precision%29))
  (bind _returnvalue (Transformation|GetActorLocation))
  (bind _returnvalue_2 (Transformation|GetActorForwardVector))
  (bind _distance (Variables|Default|GetDistance))
  (bind _returnvalue_3 (* _returnvalue_2 _distance))
  (bind _returnvalue_4 (+ _returnvalue _returnvalue_3))
  (Variables|Default|SetTraceEnd _returnvalue_4)
  (bind _outhit (Collision|LineTraceByChannel _returnvalue _returnvalue_4 "TraceTypeQuery2" false 0 "ForOneFrame"))
  (Variables|Default|SetHasHit (.bBlockingHit (Collision|BreakHitResult _outhit)))
  (Variables|Default|SetHitLocation (.ImpactPoint (Collision|BreakHitResult _outhit)))
  (Effects|Components|ParticleSystem|SetVectorParameter (Variables|Default|GetLaser) "LaserEnd" (select (Variables|Default|GetHasHit) (Variables|Default|GetHitLocation) (Variables|Default|GetTraceEnd)))
  (Rendering|SetVisibility (Variables|Default|GetLaserImpact) (Variables|Default|GetHasHit) false)
  (Transformation|SetWorldLocation (Variables|Default|GetLaserImpact) (Variables|Default|GetHitLocation) false false))

(fn ConstructionScript)