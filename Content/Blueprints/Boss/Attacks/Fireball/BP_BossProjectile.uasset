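; Boss fireball projectile that hangs in place facing the player, then fires itself after a random delay of a few seconds.
; Tick aims it at the player until launch, which stops tracking, swaps the Fireball effect from summon to trail, and sets a fast straight velocity.
; Overlapping a Player-tagged actor applies damage and starts a short lifespan.
; The line trace at launch has no effect, as its result is unused.
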(event Custom|LaunchAttack
  (bind _fireball (Variables|Default|GetFireball))
  (Actor|Tick|SetActorTickEnabled false)
  (bind _outhit (Collision|LineTraceByChannel (Transformation|GetActorLocation) (Transformation|GetActorLocation (Game|GetPlayerCharacter 0)) "TraceTypeQuery1" false 0 "None"))
  (Niagara|SetNiagaraVariable(Float) _fireball "User.TrailRate" 1.0)
  (Niagara|SetNiagaraVariable(Float) _fireball "User.SummonRate" 0.0)
  (Variables|/Script/Engine.MovementComponent|SetVelocity (Variables|Default|GetProjectileMovement) (* 3.5e+03 (Math|Vector|GetForwardVector (Variables|Default|GetFireball)))))

(event EventBeginPlay
  (Utilities|FlowControl|Delay (Math|Random|RandomFloatinRange 2.0 5.0))
  (CallFunction|LaunchAttack))

(event EventTick
  (params (DeltaSeconds :type Float%20%28single-precision%29))
  (bind _returnvalue (Transformation|GetActorLocation))
  (bind _returnvalue_2 (Game|GetPlayerCharacter 0))
  (bind _returnvalue_3 (Transformation|GetActorLocation _returnvalue_2))
  (bind _returnvalue_4 (Math|Rotator|FindLookatRotation _returnvalue _returnvalue_3))
  (Transformation|SetActorRotation (Math|Rotator|MakeRotator (.roll _returnvalue_4) (.pitch _returnvalue_4) (.yaw _returnvalue_4))))

(event Collision|EventActorBeginOverlap
  (params (OtherActor :type Actor%20Object%20Reference))
  (if (Actor|ActorHasTag OtherActor "Player")
    (Game|Damage|ApplyDamage OtherActor 5e+01 0 0)
    (Actor|SetLifeSpan 1.0)))

(fn ConstructionScript)