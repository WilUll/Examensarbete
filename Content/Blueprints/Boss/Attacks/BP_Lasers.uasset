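; BP_Lasers is a boss attack actor with two lasers that slide back and forth and a mesh that can spin.
; From BeginPlay, each laser waits a random delay, then eases between two position markers via the MoveLaser macro, with Laser2's completion restarting both branches.
; Tick optionally yaws the static mesh in either direction at RotSpeed.
; ActivateLasers only toggles visibility of BPLaser and BPLaser1, without stopping movement.
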(event EventBeginPlay
  (Utilities|FlowControl|Sequence :!label _label
    (:then_0
      (Utilities|FlowControl|Delay (Math|Random|RandomFloatinRange 0.0 3.0))
      (Utilities|MoveLaser (Variables|Default|GetLaser1) (Variables|/Script/Engine.SceneComponent|GetRelativeLocation (Variables|Default|GetLaserPos1)) (Variables|/Script/Engine.SceneComponent|GetRelativeLocation (Variables|Default|GetLaserPos2))))
    (:then_1
      (Utilities|FlowControl|Delay (Math|Random|RandomFloatinRange 0.0 3.0))
      (Utilities|MoveLaser (Variables|Default|GetLaser2) (Variables|/Script/Engine.SceneComponent|GetRelativeLocation (Variables|Default|GetLaserPos3)) (Variables|/Script/Engine.SceneComponent|GetRelativeLocation (Variables|Default|GetLaserPos4))
        (:Out
          (goto _label))))))

(event Collision|EventActorBeginOverlap
  (params (OtherActor :type Actor%20Object%20Reference)))

(event EventTick
  (params (DeltaSeconds :type Float%20%28single-precision%29))
  (bind _staticmesh (Variables|Default|GetStaticMesh))
  (bind _rotspeed (Variables|Default|GetRotSpeed))
  (bind _returnvalue (Transformation|GetWorldRotation _staticmesh))
  (bind _returnvalue_2 (* DeltaSeconds _rotspeed))
  (bind (_roll _pitch _yaw) (Math|Rotator|BreakRotator _returnvalue))
  (if (Variables|Default|GetShouldRotate)
    (if (Variables|Default|GetRotateRight)
      (Transformation|SetWorldRotation _staticmesh (Math|Rotator|MakeRotator _roll _pitch (+ _yaw _returnvalue_2)) false false)
      (else
        (Transformation|SetWorldRotation _staticmesh (Math|Rotator|MakeRotator _roll _pitch (- _yaw _returnvalue_2)) false false)))))

(fn ConstructionScript)

(fn ActivateLasers
  (params (IsActive :type Boolean))
  (Development|SetHiddeninGame (Variables|Default|GetBP_Laser1) (not IsActive) false))