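; A boss attack pillar that moves out along a timeline, retracts and then destroys itself.
; On spawn it gets a random yaw, and the timeline drives the mesh's relative location with a continuous camera shake and a one-time, delayed rock-break sound.
; A FlipFlop on timeline completion triggers the delayed reverse, then destruction.
; Player overlap with the box launches the character upward with random sideways velocity and applies damage.
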(event OnComponentBeginOverlap(Box)
  (params (OverlappedComponent :type Primitive%20Component%20Object%20Reference) (OtherActor :type Actor%20Object%20Reference) (OtherComp :type Primitive%20Component%20Object%20Reference) (OtherBodyIndex :type Integer) (bFromSweep :type Boolean) (SweepResult :type Hit%20Result%20Structure%20%28by%20ref%29))
  (bind _returnvalue (Game|Player|GetPlayerPawn 0))
  (if (== OtherActor _returnvalue)
    (Character|LaunchCharacter (Game|GetPlayerCharacter 0) (Math|Vector|MakeVector (Math|Random|RandomFloatinRange -5e+02 5e+02) (Math|Random|RandomFloatinRange -5e+02 5e+02) 1e+03) false false)
    (Game|Damage|ApplyDamage _returnvalue 1e+01 0 0)))

(event EventBeginPlay
  (Transformation|SetRelativeRotation (Variables|Default|GetStaticMesh) (Math|Rotator|MakeRotator 0.0 0.0 (Math|Random|RandomFloatinRange 0.0 3.6e+02)) false false)
  (bind _newtrack_1 (Timeline|Timeline_0 PlayFromStart)
    (:Update
      (Camera|PlayWorldCameraShake "/Game/Blueprints/Boss/BehaviourTrees/BossCameraShake.BossCameraShake_C" (Transformation|GetActorLocation) 1.0 5e+02)
      (Transformation|SetRelativeLocation (Variables|Default|GetStaticMesh) _newtrack_1 false false)
      (Utilities|FlowControl|DoOnce false
        (:Completed
          (Utilities|FlowControl|Delay 0.239164)
          (Audio|PlaySoundatLocation "/Game/SoundEffekts/631485__newlocknew__rockbrk-stone-hit-shattering-into-fragments-em-7lrs.631485__newlocknew__rockbrk-stone-hit-shattering-into-fragments-em-7lrs" (Transformation|GetActorLocation) "0, 0, 0" 1.0 1.0 0.0 0 0 0 0))))
    (:Finished
      (Utilities|FlowControl|FlipFlop
        (:A
          (Utilities|FlowControl|Delay 0.1)
          (Timeline|Timeline_0 ReverseFromEnd))
        (:B
          (Actor|DestroyActor))))))

(fn ConstructionScript)