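; BP_AmmoPickup is an ammo pickup that refills the player's weapon reserves and then disappears.
; An ActorSequence animation loops indefinitely from BeginPlay.
; When the player character overlaps the Box, it adds a fixed amount to CurrentReserve on every entry in BP_Player's Weapon array, with no cap here.
; The reload sound plays inside that loop, once per weapon, before the actor destroys itself.
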(event OnComponentBeginOverlap(Box)
  (params (OverlappedComponent :type Primitive%20Component%20Object%20Reference) (OtherActor :type Actor%20Object%20Reference) (OtherComp :type Primitive%20Component%20Object%20Reference) (OtherBodyIndex :type Integer) (bFromSweep :type Boolean) (SweepResult :type Hit%20Result%20Structure%20%28by%20ref%29))
  (bind _returnvalue (Game|GetPlayerCharacter 0))
  (if (== OtherActor _returnvalue)
    (bind _asbp_player (Utilities|Casting|CastToBP_Player _returnvalue))
    (for _array_element (Variables|/Script/Examensarbete.FPSCharacter|GetWeapon _asbp_player)
      (Variables|/Script/Examensarbete.Weapon|SetCurrentReserve _array_element (+ (Variables|/Script/Examensarbete.Weapon|GetCurrentReserve _array_element) 30))
      (Audio|PlaySoundatLocation "/Game/FPSweapon/Sounds/ReloadPistol.ReloadPistol" (Transformation|GetActorLocation) "0, 0, 0" 1.0 1.0 0.0 0 0 0 0))
    (Actor|DestroyActor)))

(event EventBeginPlay
  (Class|MovieSceneSequencePlayer|PlayLooping (Variables|/Script/ActorSequence.ActorSequenceComponent|GetSequencePlayer (Variables|Default|GetActorSequence)) -1))

(event Collision|EventActorBeginOverlap
  (params (OtherActor :type Actor%20Object%20Reference)))

(event EventTick
  (params (DeltaSeconds :type Float%20%28single-precision%29)))

(fn ConstructionScript)