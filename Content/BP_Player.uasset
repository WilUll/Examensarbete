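; Player Blueprint that plays footstep sounds while the player moves horizontally with zero vertical velocity.
; Tick checks velocity against a small threshold and, through a DoOnce, starts a looping timer at the footstep interval.
; The timer plays the step sound below the actor's location with randomized pitch.
; When the movement condition fails, Tick clears the timer and resets the DoOnce.
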(event Custom|PlayFootstep
  (Audio|PlaySoundatLocation "/Game/SoundEffekts/Footsteps/Steps.Steps" (- (Transformation|GetActorLocation) "0,0,44.000000") "0, 0, 0" 1.0 (Math|Random|RandomFloatinRange 0.8 1.2) 0.0 0 0 0 0))

(event EventBeginPlay)

(event Collision|EventActorBeginOverlap
  (params (OtherActor :type Actor%20Object%20Reference)))

(event EventTick
  (params (DeltaSeconds :type Float%20%28single-precision%29))
  (bind _returnvalue (Transformation|GetVelocity))
  (if (and (Math|Boolean|ORBoolean (> (.x _returnvalue) 2.0) (< (.x _returnvalue) -2.0) (> (.y _returnvalue) 2.0) (< (.y _returnvalue) -2.0)) (== (.z _returnvalue) 0.0))
    (Utilities|FlowControl|DoOnce false :!label _label
      (:Completed
        (bind _returnvalue_2 (Utilities|Time|SetTimerbyEvent (delegate Custom|PlayFootstep) (Variables|Default|GetFootstepInterval) true))))
    (else
      (Utilities|Time|ClearandInvalidateTimerbyHandle _returnvalue_2)
      (goto _label Reset))))

(fn ConstructionScript)