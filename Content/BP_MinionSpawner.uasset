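; Minion spawner actor that periodically creates actors of a configurable minion class at its SpawnLocation component.
; BeginPlay starts a looping timer at the SpawnTimer interval, which fires SpawnMinions.
; That event loops over AmountToSpawn with a TimeBetweenSpawns Delay before SpawnActor.
; The Delay sits inside a plain for loop, which does not wait on latent nodes, so spawns are not actually staggered.
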(event Custom|SpawnMinions
  (for _index (range 0 (Variables|Default|GetAmountToSpawn))
    (Utilities|FlowControl|Delay (Variables|Default|GetTimeBetweenSpawns))
    (Game|SpawnActorfromClass (Variables|Default|GetMinionToSpawn) (Math|Transform|MakeTransform (Transformation|GetWorldLocation (Variables|Default|GetSpawnLocation)) "0, 0, 0" "1.000000,1.000000,1.000000") "Undefined" 0 0)))

(event EventBeginPlay
  (Utilities|Time|SetTimerbyEvent (delegate Custom|SpawnMinions) (Variables|Default|GetSpawnTimer) true))

(event Collision|EventActorBeginOverlap
  (params (OtherActor :type Actor%20Object%20Reference)))

(event EventTick
  (params (DeltaSeconds :type Float%20%28single-precision%29)))

(fn ConstructionScript)